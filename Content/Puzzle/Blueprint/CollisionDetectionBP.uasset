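; CollisionDetectionBP is a puzzle trigger actor that reacts when a designated incoming piece overlaps it.
; On a matching overlap it records the target piece's location, destroys that piece and spawns an explosion particle effect there.
; It then destroys itself, so the reaction fires only once.
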(event EventBeginPlay)

(event EventActorBeginOverlap
  (params (OtherActor :type Actor%20Object%20Reference))
  (if (== OtherActor (Variables|Default|GetincomingPiece))
    (Variables|Default|SetWorldLoc (Transformation|GetActorLocation (Variables|Default|GettargetPiece)))
    (Actor|DestroyActor (Variables|Default|GettargetPiece))
    (Effects|SpawnEmitteratLocation "/Game/StarterContent/Particles/P_Explosion.P_Explosion" (Variables|Default|GetWorldLoc))
    (Actor|DestroyActor self)))

(event EventTick
  (params (DeltaSeconds :type Float%20%28single-precision%29)))

(fn ConstructionScript)